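; BP_Course runs a timed checkpoint course from a starting point through a set of checkpoints.
; Reaching the start sets the course active and shows a timer widget, while each checkpoint adds seconds and the last finishes the course.
; Tick uses a one-second Delay to count down and refresh the minutes:seconds display.
; InitCourse deactivates checkpoints, reactivates the start and clears widgets on construction, BeginPlay, finish or time-out.
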(event `self.ReceiveTick`
  (params (DeltaSeconds :type "Float (single-precision)"))
  (`KismetSystemLibrary.Delay` 1.0)
  (if (== (`self.Timer`) 0)
    (`KismetSystemLibrary.PrintString` "Time over")
    (set `self.IsActive` false)
    (`self.InitCourse`)
    (else
      (`/Engine/EditorBlueprintResources/StandardMacros.DecrementInt` (`self.Timer`)
        (:`  `
          (`self.UpdateTimerWidget`))))))

(event `self.ReceiveBeginPlay`
  (`self.InitCourse`)
  (add `/Game/Blueprints/BP_Checkpoint.On Checkpoint Reached` (`self.StartingPoint`) (delegate `Start Course`))
  (for _array_element (`self.Checkpoints`)
    (add `/Game/Blueprints/BP_Checkpoint.On Checkpoint Reached` _array_element (delegate `Checkpoint Reached`))))

(event `Checkpoint Reached`
  (params (IsLast :type Boolean) (SecondsToAdd :type Integer))
  (if IsLast
    (`KismetSystemLibrary.PrintString` "Course Finished")
    (`self.InitCourse`)
    (else
      (`KismetSystemLibrary.PrintString` "Checkpoint Reached!")
      (set `self.Timer` (+ SecondsToAdd (`self.Timer`)))
      (`self.UpdateTimerWidget`))))

(event `Start Course`
  (params (IsLast :type Boolean) (SecondsToAdd :type Integer))
  (set `self.IsActive` true)
  (set `self.Timer` 0)
  (bind _returnvalue (`|CreateWidget` "/Game/Blueprints/Timer.Timer_C"))
  (bind _output_get (set `self.TimerWidget` _returnvalue))
  (`UserWidget.AddToViewport` _output_get 0))

(fn `InitCourse`
  (for _array_element (`self.Checkpoints`)
    (`/Game/Blueprints/BP_Checkpoint.On Deactivate` _array_element))
  (`/Game/Blueprints/BP_Checkpoint.On Activate` (`self.StartingPoint`))
  (set `self.Timer` -1)
  (`WidgetLayoutLibrary.RemoveAllWidgets`))

(fn `UpdateTimerWidget`
  (bind _timer (`self.Timer`))
  (`/Engine/EditorBlueprintResources/StandardMacros.IsValid` (`self.TimerWidget`)
    (:`Is Valid`
      (`/Game/Blueprints/Timer.UpdateText_Event` (`self.TimerWidget`) (`KismetStringLibrary.Concat_StrStr` (`KismetTextLibrary.Conv_TextToString` (`KismetTextLibrary.Conv_IntToText` (/ _timer 60) false true 2)) ":" (`KismetTextLibrary.Conv_TextToString` (`KismetTextLibrary.Conv_IntToText` (mod _timer 60) false true 2)))))))

(fn `UserConstructionScript`
  (`self.InitCourse`))