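; BP_Checkpoint is a chained checkpoint actor, visible while active, that the player reaches by entering its trigger sphere.
; On overlap by the player pawn, it deactivates, fires a CheckpointReached dispatcher for the Level Blueprint with a last-checkpoint flag and seconds to add, then activates NextCheckpoint if valid.
; It hides once the player leaves the sphere, and the construction script sets initial visibility from IsActive.
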(event `On Activate`
  ;[0.05098 0.05098 0.05098] Activate Checkpoint
  (set `self.IsActive` true)
  (`self.SetActorHiddenInGame` false))

(event `On Deactivate`
  (set `self.IsActive` false)
  (`self.SetActorHiddenInGame` true))

(event `self.TriggerSphere.OnComponentBeginOverlap`
  (params (OverlappedComponent :type "PrimitiveComponent Object Reference") (OtherActor :type "Actor Object Reference") (OtherComp :type "PrimitiveComponent Object Reference") (OtherBodyIndex :type Integer) (bFromSweep :type Boolean) (SweepResult :type "HitResult Structure (by ref)"))
  (bind _nextcheckpoint (`self.NextCheckpoint`))
  (bind _returnvalue (`KismetSystemLibrary.IsValid` _nextcheckpoint))
  ;[0.05098 0.05098 0.05098] Checkpoint Reached Handling - Activate next checkpoint and send a "Checkpoint Reached" event to the Level BP
  (if (and (`self.IsActive`) (== OtherActor (`GameplayStatics.GetPlayerPawn` 0)))
    (set `self.IsActive` false)
    (`self.On Checkpoint Reached` (not _returnvalue) (`self.NextCheckpointTime`))
    (if _returnvalue
      (`self.On Activate` _nextcheckpoint))))

(event `self.TriggerSphere.OnComponentEndOverlap`
  (params (OverlappedComponent :type "PrimitiveComponent Object Reference") (OtherActor :type "Actor Object Reference") (OtherComp :type "PrimitiveComponent Object Reference") (OtherBodyIndex :type Integer))
  ;[0.05098 0.05098 0.05098] Hide Checkpoint After Reached
  (if (and (not (`self.IsActive`)) (== OtherActor (`GameplayStatics.GetPlayerPawn` 0)))
    (`self.SetActorHiddenInGame` true)))

(fn `UserConstructionScript`
  (if (`self.IsActive`)
    (`self.SetActorHiddenInGame` false)
    (else
      (`self.SetActorHiddenInGame` true))))